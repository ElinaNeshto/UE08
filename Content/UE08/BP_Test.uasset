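; BP_Test is a test Blueprint that sketches a purchase decision, mostly with placeholder logic.
; On BeginPlay it branches on IsEnoughMoney, calling MakePurchase and deducting TotalCost from Money, or calling ReturnToWork.
; MakePurchase and ReturnToWork are empty, and TotalCost returns zero, so the deduction changes nothing.
; SumOfTwo feeds TotalCost but leaves its addition unused, and the NodsName node is never executed.
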(event EventBeginPlay
  (if (Variables|Default|GetIsEnoughMoney)
    (CallFunction|MakePurchase)
    (bind _itog (CallFunction|TotalCost (Utilities|SumOfTwo 10 20)))
    (Variables|Default|SetMoney (- (Variables|Default|GetMoney) _itog))
    (else
      (CallFunction|ReturntoWork))))

(event Collision|EventActorBeginOverlap
  (params (OtherActor :type Actor%20Object%20Reference)))

(event EventTick
  (params (DeltaSeconds :type Float%20%28single-precision%29)))

(fn ConstructionScript)

(fn MakePurchase)

(fn ReturntoWork)

(fn TotalCost
  (params (Money :type Integer))
  (return 0))