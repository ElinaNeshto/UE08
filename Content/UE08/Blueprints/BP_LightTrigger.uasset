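; BP_LightTrigger is a trigger volume that changes a point light's color when a twin-stick character enters or leaves it.
; Box overlap events cast the other actor to BP_TwinStickCharacter and set the IsActorEntered flag.
; Both events share one branch on that flag, turning PointLight green on entry and red on exit.
; BeginPlay holds only a switch on a constant Pistol value with no actions.
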(event OnComponentBeginOverlap(Box)
  (params (OverlappedComponent :type Primitive%20Component%20Object%20Reference) (OtherActor :type Actor%20Object%20Reference) (OtherComp :type Primitive%20Component%20Object%20Reference) (OtherBodyIndex :type Integer) (bFromSweep :type Boolean) (SweepResult :type Hit%20Result%20Structure%20%28by%20ref%29))
  (Utilities|Casting|CastToBP_TwinStickCharacter OtherActor)
  (if true
    (Variables|Default|SetIsActorEntered true)
    (if (Variables|Default|GetIsActorEntered)
      (Rendering|Components|Light|SetLightColor (Variables|Default|GetPointLight) "(R=0.152526,G=1.000000,B=0.073879,A=1.000000)" true)
      (else
        (Rendering|Components|Light|SetLightColor (Variables|Default|GetPointLight) "(R=1.000000,G=0.000000,B=0.000000,A=1.000000)" true)))))

(event OnComponentEndOverlap(Box)
  (params (OverlappedComponent :type Primitive%20Component%20Object%20Reference) (OtherActor :type Actor%20Object%20Reference) (OtherComp :type Primitive%20Component%20Object%20Reference) (OtherBodyIndex :type Integer))
  (Utilities|Casting|CastToBP_TwinStickCharacter OtherActor)
  (if true
    (Variables|Default|SetIsActorEntered false)
    (if (Variables|Default|GetIsActorEntered)
      (Rendering|Components|Light|SetLightColor (Variables|Default|GetPointLight) "(R=0.152526,G=1.000000,B=0.073879,A=1.000000)" true)
      (else
        (Rendering|Components|Light|SetLightColor (Variables|Default|GetPointLight) "(R=1.000000,G=0.000000,B=0.000000,A=1.000000)" true)))))

(event EventBeginPlay
  (switch Utilities|FlowControl|Switch|SwitchonE_ItemType "NewEnumerator0"))

(fn ConstructionScript)